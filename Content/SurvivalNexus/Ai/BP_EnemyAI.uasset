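; BP_EnemyAI is an enemy that chases the player and is destroyed when it overlaps a Magic_Bullet.
; PawnSensing's OnSeePawn sets IsSeeingPlayer without checking which pawn was seen, then calls FollowPlayer.
; FollowPlayer issues an AIMoveTo targeting player character 0, with no behavior tree.
; IsSeeingPlayer is never cleared here, and movement is only requested on sight events.
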(event `self.ReceiveActorBeginOverlap`
  (params (OtherActor :type "Actor Object Reference"))
  (cast `/Game/SurvivalNexus/Blueprints/Magic_Bullet` OtherActor)
  (`self.K2_DestroyActor`))

(event `self.PawnSensing.OnSeePawn`
  (params (Pawn :type "Pawn Object Reference"))
  (set `self.IsSeeingPlayer` true)
  (`self.FollowPlayer`))

(event `FollowPlayer`
  (bind _returnvalue (`GameplayStatics.GetPlayerCharacter` 0))
  (if (`self.IsSeeingPlayer`)
    (`|AIMoveTo` self (`SceneComponent.K2_GetComponentLocation` (`Character.Mesh` _returnvalue)) _returnvalue)))

(fn `UserConstructionScript`)