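; BP_CraftingStation is a crafting station that combines a wood and a stone item held in two slots.
; Craft reads each slot's GrabActor and uses two cast chains in a sequence to accept the pair in either order.
; A match immediately spawns a BP_Wood at the station mesh's location and starts a short timer that calls EmptyItems to destroy both ingredients.
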(event `Craft`
  (bind _returnvalue (`SceneComponent.K2_GetComponentLocation` (`self.StaticMesh`)))
  (set `self.Item1` (`/Game/SurvivalNexus/Blueprints/Station_Component.GrabActor` (`self.Slot1`)))
  (set `self.Item2` (`/Game/SurvivalNexus/Blueprints/Station_Component.GrabActor` (`self.Slot2`)))
  (`|ExecutionSequence`
    (:`then_0`
      (cast `/Game/SurvivalNexus/Blueprints/BP_Wood` (`self.Item1`))
      (cast `/Game/SurvivalNexus/Blueprints/BP_Stone` (`self.Item2`))
      (`KismetSystemLibrary.K2_SetTimerDelegate` (delegate `EmptyItems`) 3.0)
      (`|SpawnActorFromClass` "/Game/SurvivalNexus/Blueprints/BP_Wood.BP_Wood_C" (`KismetMathLibrary.MakeTransform` _returnvalue) "Undefined" "MultiplyWithRoot" null null))
    (:`then_1`
      (cast `/Game/SurvivalNexus/Blueprints/BP_Stone` (`self.Item1`))
      (cast `/Game/SurvivalNexus/Blueprints/BP_Wood` (`self.Item2`))
      (`KismetSystemLibrary.K2_SetTimerDelegate` (delegate `EmptyItems`) 3.0)
      (`|SpawnActorFromClass` "/Game/SurvivalNexus/Blueprints/BP_Wood.BP_Wood_C" (`KismetMathLibrary.MakeTransform` _returnvalue) "Undefined" "MultiplyWithRoot" null null))))

(event `EmptyItems`
  (`self.K2_DestroyActor` (`self.Item1`))
  (`self.K2_DestroyActor` (`self.Item2`)))

(fn `UserConstructionScript`)