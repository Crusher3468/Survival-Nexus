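; VR Codex that the player grabs with a motion controller and that carries a toggleable nine-slot inventory.
; Grab snaps it to the controller and shows it, while Release from the holding controller returns it to DefaultComponent, if valid, and hides it.
; OpenInventory flips inventory visibility and each slot's InvOpen flag, which start off in the construction script.
; The Active function reports whether the Codex is held.
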(event `/Game/SurvivalNexus/Interfaces/Grab.Grab`
  (params (`Motion Controller` :type "MotionControllerComponent Object Reference"))
  (bind _output_get (set `self.Motion Controller` `Motion Controller`))
  (`self.K2_AttachToComponent` _output_get "None" "SnapToTarget" "SnapToTarget" "KeepWorld")
  (`SceneComponent.SetHiddenInGame` (`self.Codex`) false true)
  (`PrimitiveComponent.SetCastShadow` (`self.Codex`) true)
  (set `self.CodexActive` true))

(event `/Game/SurvivalNexus/Interfaces/Grab.Release`
  (params (`Motion Controller` :type "MotionControllerComponent Object Reference"))
  (if (== `Motion Controller` (`self.Motion Controller`))
    (set `self.Motion Controller` null)
    (bind _defaultcomponent (`self.DefaultComponent`)
      (:`then`
        (`self.K2_AttachToComponent` _defaultcomponent "None" "SnapToTarget" "SnapToTarget" "KeepWorld")
        (`SceneComponent.SetHiddenInGame` (`self.Codex`) true true)
        (`PrimitiveComponent.SetCastShadow` (`self.Codex`) false)
        (set `self.CodexActive` false))
      (:`else`))))

(event `OpenInventory`
  (bind _inventory (`self.Inventory`))
  (if (`self.InventoryActive`)
    (`SceneComponent.SetVisibility` _inventory false true)
    (`self.SetSlotsInactive`)
    (set `self.InventoryActive` false)
    (else
      (`SceneComponent.SetVisibility` _inventory true true)
      (`self.SetSlotsActive`)
      (set `self.InventoryActive` true))))

(fn `Active`
  (returns (IsActive :type Boolean))
  (return (`self.CodexActive`)))

(fn `SetSlotsActive`
  (set `/Game/SurvivalNexus/Blueprints/Inventory_Component.InvOpen` true (`self.Slot 7`))
  (set `/Game/SurvivalNexus/Blueprints/Inventory_Component.InvOpen` true (`self.Slot 9`))
  (set `/Game/SurvivalNexus/Blueprints/Inventory_Component.InvOpen` true (`self.Slot 8`))
  (set `/Game/SurvivalNexus/Blueprints/Inventory_Component.InvOpen` true (`self.slot 4`))
  (set `/Game/SurvivalNexus/Blueprints/Inventory_Component.InvOpen` true (`self.slot 6`))
  (set `/Game/SurvivalNexus/Blueprints/Inventory_Component.InvOpen` true (`self.slot 5`))
  (set `/Game/SurvivalNexus/Blueprints/Inventory_Component.InvOpen` true (`self.Slot 2`))
  (set `/Game/SurvivalNexus/Blueprints/Inventory_Component.InvOpen` true (`self.Slot 3`))
  (set `/Game/SurvivalNexus/Blueprints/Inventory_Component.InvOpen` true (`self.Slot 1`)))

(fn `SetSlotsInactive`
  (set `/Game/SurvivalNexus/Blueprints/Inventory_Component.InvOpen` false (`self.Slot 7`))
  (set `/Game/SurvivalNexus/Blueprints/Inventory_Component.InvOpen` false (`self.Slot 9`))
  (set `/Game/SurvivalNexus/Blueprints/Inventory_Component.InvOpen` false (`self.Slot 8`))
  (set `/Game/SurvivalNexus/Blueprints/Inventory_Component.InvOpen` false (`self.slot 4`))
  (set `/Game/SurvivalNexus/Blueprints/Inventory_Component.InvOpen` false (`self.slot 6`))
  (set `/Game/SurvivalNexus/Blueprints/Inventory_Component.InvOpen` false (`self.slot 5`))
  (set `/Game/SurvivalNexus/Blueprints/Inventory_Component.InvOpen` false (`self.Slot 2`))
  (set `/Game/SurvivalNexus/Blueprints/Inventory_Component.InvOpen` false (`self.Slot 3`))
  (set `/Game/SurvivalNexus/Blueprints/Inventory_Component.InvOpen` false (`self.Slot 1`)))

(fn `UserConstructionScript`
  (`SceneComponent.SetVisibility` (`self.Codex`) false false)
  (`PrimitiveComponent.SetCastShadow` (`self.Codex`) false)
  (`SceneComponent.SetVisibility` (`self.Inventory`) false true)
  (`self.SetSlotsInactive`))