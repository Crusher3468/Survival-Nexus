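; Inventory Blueprint that starts hidden in game and exposes an Activated flag through its Active function.
; Its construction script hides the root and all children.
; When Activated is false, ShowInv sets it to false again, finds the Codex actor and calls a snap-to-target component attach that keeps world scale.
; Nothing here unhides it or sets the flag true, and a validity-checked attach to DefaultComponent is left unconnected.
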(event `ShowInv`
  (if (not (`self.Activated`))
    (set `self.Activated` false)
    (bind _returnvalue (`GameplayStatics.GetActorOfClass` "/Game/SurvivalNexus/Blueprints/Codex.Codex_C"))
    (`self.K2_AttachToComponent` _returnvalue null "None" "SnapToTarget" "SnapToTarget" "KeepWorld" true)))

(fn `Active`
  (returns (IsActive :type Boolean))
  (return (`self.Activated`)))

(fn `UserConstructionScript`
  (`SceneComponent.SetHiddenInGame` (`self.DefaultSceneRoot`) true true))